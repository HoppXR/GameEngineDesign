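; Game manager Blueprint that tracks a current count against a total and triggers the win state when the target is reached.
; It creates the WBP_Count HUD, exposes events to grow the total, add progress or reset both counters, and refreshes the counter text.
; Each progress increment runs the win check, which reveals the win text and Play Again and Quit buttons, shows the cursor and pauses the game.
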(event Custom|AddCount
  (Math|Integer|IncrementInt (Variables|Default|GetCurrentCount)
    (:%20%20
      (CallFunction|UpdateCount)
      (CallFunction|GameWin))))

(event Custom|GameWin
  (bind _countwidget (Variables|Default|GetCountWidget))
  (if (>= (Variables|Default|GetCurrentCount) (Variables|Default|GetTotalCount))
    (Widget|SetVisibility (Variables|/Game/Blueprints/WBP_Count.WBP_Count_C|GetWinText _countwidget) "Visible")
    (Widget|SetVisibility (Variables|/Game/Blueprints/WBP_Count.WBP_Count_C|GetPlayAgainButton _countwidget) "Visible")
    (Widget|SetVisibility (Variables|/Game/Blueprints/WBP_Count.WBP_Count_C|GetQuitButton _countwidget) "Visible")
    (Variables|/Script/Engine.PlayerController|SetbShowMouseCursor (Game|GetPlayerController 0) true)
    (Game|SetGamePaused true)))

(event Custom|AddTotalCount
  (Math|Integer|IncrementInt (Variables|Default|GetTotalCount)))

(event Custom|AddUI
  (bind _returnvalue (UserInterface|CreateWidget "/Game/Blueprints/WBP_Count.WBP_Count_C"))
  (bind _output_get (Variables|Default|SetCountWidget _returnvalue))
  (UserInterface|Viewport|AddtoViewport _output_get 0)
  (CallFunction|UpdateCount))

(event Custom|UpdateCount
  (Rendering|Components|TextRender|SetText (Variables|/Game/Blueprints/WBP_Count.WBP_Count_C|GetCountText (Variables|Default|GetCountWidget)) (Utilities|Text|FormatText "{Amount} / {Total}" (Variables|Default|GetCurrentCount) (Variables|Default|GetTotalCount))))

(event Custom|ResetCount
  (Variables|Default|SetTotalCount 0)
  (Variables|Default|SetCurrentCount 0))