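; Spawner Blueprint that drops collectable orbs at random X/Y positions within a square area around the world origin.
; Each spawner event calls an RNG event that rolls a weighted rarity tier from Common to Legendary, then spawns that orb class.
; A second independent roll occasionally also spawns a bomb orb at another random position, reusing the same class variable.
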(event Custom|CollectableSpawnerEvent
  (CallFunction|RNG)
  (Game|SpawnActorfromClass (Variables|Default|GetCollectableClass) (Math|Transform|MakeTransform (Math|Vector|MakeVector (Math|Random|RandomFloatinRange -1e+03 1e+03) (Math|Random|RandomFloatinRange -1e+03 1e+03) 0.0)) "Undefined" "MultiplyWithRoot" 0 0)
  (if (>= (Math|Random|RandomIntegerinRange 0 100) 80)
    (bind _output_get (Variables|Default|SetCollectableClass "/Game/Blueprints/Factory/BP_BombOrb.BP_BombOrb_C"))
    (Game|SpawnActorfromClass _output_get (Math|Transform|MakeTransform (Math|Vector|MakeVector (Math|Random|RandomFloatinRange -1e+03 1e+03) (Math|Random|RandomFloatinRange -1e+03 1e+03) 0.0)) "Undefined" "MultiplyWithRoot" 0 0)))

(event Custom|RNG
  (Variables|Default|SetRandomNumber (Math|Random|RandomIntegerinRange 0 100))
  (if (>= (Variables|Default|GetRandomNumber) 95)
    (Variables|Default|SetCollectableClass "/Game/Blueprints/Factory/BP_LegendaryOrb.BP_LegendaryOrb_C")
    (elif (>= (Variables|Default|GetRandomNumber) 85)
      (Variables|Default|SetCollectableClass "/Game/Blueprints/Factory/BP_EpicOrb.BP_EpicOrb_C")
      (elif (>= (Variables|Default|GetRandomNumber) 70)
        (Variables|Default|SetCollectableClass "/Game/Blueprints/Factory/BP_RareOrb.BP_RareOrb_C")
        (elif (>= (Variables|Default|GetRandomNumber) 55)
          (Variables|Default|SetCollectableClass "/Game/Blueprints/Factory/BP_UncommonOrb.BP_UncommonOrb_C")
          (else
            (Variables|Default|SetCollectableClass "/Game/Blueprints/Factory/BP_CommonOrb.BP_CommonOrb_C")))))))

(fn ConstructionScript)